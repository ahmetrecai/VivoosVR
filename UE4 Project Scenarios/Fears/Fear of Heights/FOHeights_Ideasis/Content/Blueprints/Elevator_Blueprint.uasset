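; Elevator actor that moves up or down one floor at a time between floor 0 and a hardcoded top floor of 12.
; GoUp and GoDown events check movement and floor limits, then lerp the actor vertically by DistanceBetweenFloors using separate timelines, with descent played in reverse.
; When each move finishes, it updates the floor count and writes it to the Elevator_Floor widget on its FloorDisplayer component.
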(event Custom|Event_GoUp
  (bind _returnvalue (Transformation|GetActorLocation))
  (bind (_x _y _z) (Math|Vector|BreakVector _returnvalue))
  ;[1 1 1] Elevator starts to go up
  ; -If it is not already moving and it is not already at the last floor (12 in this case)
  ; -Elevator_Move Timeline allows elevator to move from one point to another in 3 seconds
  (if (and (not (Variables|Default|GetisElevatorMoving)) (< (Variables|Default|GetCurrentFloor_Integer) 12))
    (Variables|Default|SetCurrentFloor _returnvalue)
    (Variables|Default|SetNextFloor (Math|Vector|MakeVector _x _y (+ _z (Variables|Default|GetDistanceBetweenFloors))))
    (Variables|Default|SetisElevatorMoving true)
    (bind _alpha (Timeline|Elevator_Move PlayFromStart)
      (:Update
        (Transformation|SetActorLocation (Math|Vector|Lerp(Vector) (Variables|Default|GetCurrentFloor) (Variables|Default|GetNextFloor) _alpha) false false))
      (:Finished
        (Variables|Default|SetisElevatorMoving false)
        (Math|Integer|IncrementInt (Variables|Default|GetCurrentFloor_Integer)
          (:%20%20
            (CallFunction|ChangeFloorDisplayer)))))))

(event Custom|Event_GoDown
  (bind _returnvalue (Transformation|GetActorLocation))
  (bind (_x _y _z) (Math|Vector|BreakVector _returnvalue))
  ;[1 1 1] Elevator starts to go down
  (if (and (not (Variables|Default|GetisElevatorMoving)) (> (Variables|Default|GetCurrentFloor_Integer) 0))
    (Variables|Default|SetCurrentFloor _returnvalue)
    (Variables|Default|SetNextFloor (Math|Vector|MakeVector _x _y (- _z (Variables|Default|GetDistanceBetweenFloors))))
    (Variables|Default|SetisElevatorMoving true)
    (bind _alpha (Timeline|Timeline_0 ReverseFromEnd)
      (:Update
        (Transformation|SetActorLocation (Math|Vector|Lerp(Vector) (Variables|Default|GetNextFloor) (Variables|Default|GetCurrentFloor) _alpha) false false))
      (:Finished
        (Variables|Default|SetisElevatorMoving false)
        (Math|Integer|DecrementInt (Variables|Default|GetCurrentFloor_Integer)
          (:%20%20
            (CallFunction|ChangeFloorDisplayer)))))))

(event EventBeginPlay
  ;[1 1 1] Initialize
  (bind _aselevator_floor (Utilities|Casting|CastToElevator_Floor (UserInterface|GetUserWidgetObject (Variables|Default|GetFloor_Displayer))))
  (Variables|Default|SetFloorDisplayer_Object _aselevator_floor))

(fn ConstructionScript)

(fn ChangeFloorDisplayer
  (Rendering|Components|TextRender|SetText (Variables|/Game/Blueprints/Elevator_Floor.Elevator_Floor_C|GetFloor_Text (Variables|Default|GetFloorDisplayer_Object)) (Utilities|Text|ToText(Integer) (Variables|Default|GetCurrentFloor_Integer))))